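; Player controller that connects each non-dedicated-server instance to an ODIN voice chat room on BeginPlay.
; On Android it checks microphone permission, requesting it if missing and joining after the callback regardless of grant result.
; It generates the room token locally from an access key, then streams captured microphone audio once joined.
; Remote media gets synth components on the controller, tracked by peer ID and destroyed on removal.
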(event `self.ReceiveBeginPlay`
  ;[1 1 1] The dedicated server doesn't need to connect to ODIN
  (if (not (`KismetSystemLibrary.IsDedicatedServer`))
    (`self.ConnectToRoom`)))

(event `ConnectToRoom`
  ;[1 1 1] Request permissions, if on mobile platform
  (switch `string` (`GameplayStatics.GetPlatformName`)
    (:`Default`
      (`self.Join Odin Room` :!label _label))
    (:`Android`
      (bind _returnvalue (`AndroidPermissionFunctionLibrary.CheckPermission` (`self.MicPermission`)))
      (if _returnvalue
        (`KismetSystemLibrary.PrintString` "Microphone Permission available." true true (struct :`G` 0.66 :`B` 1.0 :`A` 1.0) 10.0)
        (goto _label)
        (else
          (`KismetSystemLibrary.Delay` 0.2)
          (`KismetSystemLibrary.PrintString` "Microphone Permission not available, starting request" true true (struct :`G` 0.66 :`B` 1.0 :`A` 1.0) 10.0)
          (bind _returnvalue_2 (`AndroidPermissionFunctionLibrary.AcquirePermissions` (`|MakeArray` (`self.MicPermission`))))
          (add `AndroidPermissionCallbackProxy.OnPermissionsGrantedDynamicDelegate` _returnvalue_2 (delegate `OnGranted`)))))))

(event `OnGranted`
  (params (Permissions :type "Array of String (by ref)") (GrantResults :type "Array of Boolean (by ref)"))
  ;[1 1 1] Permission Request Callback
  (`KismetSystemLibrary.PrintString` "Permission Request Callback received" true true (struct :`G` 0.66 :`B` 1.0 :`A` 1.0) 10.0)
  (for (_array_element _array_index) Permissions
    (`KismetSystemLibrary.PrintText` (`|FormatText` "GrantResult for {permission} is: {result}" _array_element (`|GetArrayItem` GrantResults _array_index)) true true (struct :`G` 0.66 :`B` 1.0 :`A` 1.0) 10.0)
    (if (`KismetStringLibrary.EqualEqual_StrStr` (`self.MicPermission`) _array_element)
      (`|ExecutionSequence`
        (:`then_0`
          (break))
        (:`then_1`
          (`self.Join Odin Room`))))))

(event `Join Odin Room`
  (`|ExecutionSequence`
    (:`then_0`
      ;[1 1 1] Setup the Odin Connection by creating a new room token and
      (bind _returnvalue (`OdinTokenGenerator.GenerateRoomToken` (`OdinTokenGenerator.ConstructTokenGenerator` (`self.Access Key`)) (`self.Room Name`) "My User Id" "Default"))
      (set `self.RoomToken` _returnvalue)
      (set `self.RoomHandle` (`OdinRoom.ConstructRoom` (make `OdinApmSettings` false 0.6 0.5))))
    (:`then_1`
      ;[1 1 1] Handle On Media Added
      (add `OdinRoom.onMediaAdded` (`self.RoomHandle`) (delegate `OnMediaAdded`)))
    (:`then_2`
      ;[1 1 1] Destroy Odin Synth Component on Character, when the media stream is removed
      (add `OdinRoom.onMediaRemoved` (`self.RoomHandle`) (delegate `OnMediaRemoved`)))
    (:`then_3`
      ;[1 1 1] Join the Odin Room and handle success / failure
      (`OdinRoomJoin.JoinRoom` :`room` (`self.RoomHandle`) :`url` (`self.ServerUrl`) :`token` (`self.RoomToken`) :`onError` (delegate `OnJoinRoomError`) :`onSuccess` (delegate `OnJoinroomSuccess`)))))

(event `OnMediaAdded`
  (params (peerId :type Integer64) (media :type "OdinPlaybackMedia Object Reference") (properties :type "OdinJsonObject Object Reference") (room :type "OdinRoom Object Reference"))
  ;[1 1 1] Handle On Media Added
  (if (!= (`self.Own Peer Id`) peerId)
    (bind _returnvalue (`AddComponent|NODE_AddOdinSynthComponent-0`))
    (`OdinSynthComponent.Odin_AssignSynthToMedia` _returnvalue media)
    (`ActorComponent.Activate` _returnvalue false)
    (`BlueprintMapLibrary.Map_Add` (`self.PeerToSynth`) peerId _returnvalue)))

(event `OnMediaRemoved`
  (params (peerId :type Integer64) (media :type "OdinPlaybackMedia Object Reference") (room :type "OdinRoom Object Reference"))
  (bind (_value _returnvalue) (`BlueprintMapLibrary.Map_Find` (`self.PeerToSynth`) peerId))
  ;[1 1 1] Destroy Odin Synth Component on Character, when the media stream is removed
  (if _returnvalue
    (`/Engine/EditorBlueprintResources/StandardMacros.IsValid` _value
      (:`Is Valid`
        (`ActorComponent.K2_DestroyComponent` _value)))))

(event `OnJoinRoomError`
  (params (errorCode :type Integer64))
  ;[1 1 1] Join the Odin Room and handle success / failure
  (`KismetSystemLibrary.PrintString` "Hello"))

(event `OnJoinroomSuccess`
  (params (roomId :type String) (roomUserData :type "Array of Byte (by ref)") (customer :type String) (ownPeerId :type Integer64) (ownUserId :type String))
  ;[1 1 1] Join the Odin Room and handle success / failure
  ;;[1 1 1] On Join Room, start capturing audio and add capture stream to the Odin room.
  (set `self.Own Peer Id` ownPeerId)
  (`KismetSystemLibrary.PrintString` "Join Room Success")
  (bind _returnvalue (`OdinFunctionLibrary.CreateOdinAudioCapture`))
  (`AudioCapture.StartCapturingAudio` _returnvalue)
  (`OdinRoomAddMedia.AddMedia` (`self.RoomHandle`) (`OdinFunctionLibrary.Odin_CreateMedia` _returnvalue)))

(fn `UserConstructionScript`)